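; BP_Portals is a portal actor that teleports the player to another portal when a PlayerCharacter-tagged actor overlaps its collision.
; On BeginPlay it caches the world location and rotation of its landing zone.
; On overlap it finds the BP_Portals instance named by NewPortalLocation and passes that transform to PortalMemeManMover on the first BP_MemeMan_PT found.
; The Portal 1 and Portal 2 branches differ only in debug prints.
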(event OnComponentBeginOverlap(PortalCollision)
  (params (OverlappedComponent :type Primitive%20Component%20Object%20Reference) (OtherActor :type Actor%20Object%20Reference) (OtherComp :type Primitive%20Component%20Object%20Reference) (OtherBodyIndex :type Integer) (bFromSweep :type Boolean) (SweepResult :type Hit%20Result%20Structure%20%28by%20ref%29))
  (bind _new_portal_location (Variables|Default|GetNew%20Portal%20Location))
  (bind _new_portal_location_2 (Variables|Default|GetNew%20Portal%20Location))
  (if (Actor|ActorHasTag OtherActor "PlayerCharacter")
    (Development|PrintString "You are being teleported!")
    (if (Utilities|Enum|Equal(Enum) (Variables|BP_Portals_C|GetPortal%20Name self) (Utilities|Array|Get(acopy) (Variables|Default|GetPortal%20Names)))
      ;[1 1 1] For Portal 1
      (Development|PrintString "Portal 1 sends you to Portal 2!")
      (bind _outactors (Actor|GetAllActorsOfClass "BP_Portals_C"))
      (for _array_element _outactors
        (if (Utilities|Enum|Equal(Enum) _new_portal_location_2 (Variables|BP_Portals_C|GetPortal%20Name _array_element))
          (Development|PrintString (Utilities|String|Append "Portaling you to " (Utilities|String|ToString(Text) _new_portal_location_2)))
          (bind _outactors_2 (Actor|GetAllActorsOfClass "/Game/ThirdPersonBP/Blueprints/BP_MemeMan_PT.BP_MemeMan_PT_C"))
          (Default|PortalMemeManMover! (Utilities|Array|Get(acopy) _outactors_2) 0 0 (Variables|BP_Portals_C|GetPortal%20Location _array_element) (Variables|BP_Portals_C|GetPortal%20Rotation _array_element))))
      (else
        ;[1 1 1] For Portal 2
        (Development|PrintString "Portal 2 sends you to Portal 1!")
        (bind _outactors_3 (Actor|GetAllActorsOfClass "BP_Portals_C"))
        (for _array_element_2 _outactors_3
          (if (Utilities|Enum|Equal(Enum) _new_portal_location (Variables|BP_Portals_C|GetPortal%20Name _array_element_2))
            (Development|PrintString (Utilities|String|Append "Portaling you to " (Utilities|String|ToString(Text) _new_portal_location)))
            (bind _outactors_4 (Actor|GetAllActorsOfClass "/Game/ThirdPersonBP/Blueprints/BP_MemeMan_PT.BP_MemeMan_PT_C"))
            (Default|PortalMemeManMover! (Utilities|Array|Get(acopy) _outactors_4) 0 0 (Variables|BP_Portals_C|GetPortal%20Location _array_element_2) (Variables|BP_Portals_C|GetPortal%20Rotation _array_element_2))))))))

(event EventBeginPlay
  (bind _portal_landing_zone (Variables|Default|GetPortal%20Landing%20Zone))
  ;[1 1 1] Set the rotation and Location values
  (Variables|Default|SetPortal%20Location (Transformation|GetWorldLocation _portal_landing_zone))
  (Variables|Default|SetPortal%20Rotation (Transformation|GetWorldRotation _portal_landing_zone)))

(fn ConstructionScript)